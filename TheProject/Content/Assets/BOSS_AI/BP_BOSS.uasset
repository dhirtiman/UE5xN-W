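; BP_BOSS is a boss enemy that wanders and chases the hero on sight.
; While no enemy is seen, Tick moves it to random reachable nearby points, throttled by a Delay.
; PawnSensing detections of BP_Hero start a move toward that actor, and a retriggerable delay clears the seen flag after sightings stop.
; A spotted-sound block with a cooldown flag exists but is disconnected.
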(event OnSeePawn(PawnSensing)
  (params (Pawn :type Pawn%20Object%20Reference))
  (bind _asbp_hero (Utilities|Casting|CastToBP_Hero Pawn))
  (Utilities|FlowControl|Sequence
    (:then_0
      (Variables|Default|SetCanSeeEnemy? true)
      (AI|AIMoveTo self "0, 0, 0" _asbp_hero 5.0 false))
    (:then_1
      (Utilities|FlowControl|RetriggerableDelay 5.0)
      (Variables|Default|SetCanSeeEnemy? false))))

(event EventTick
  (params (DeltaSeconds :type Float%20%28single-precision%29))
  (if (not (Variables|Default|GetCanSeeEnemy?))
    (Utilities|FlowControl|Delay 1.3)
    (AI|AIMoveTo self (.RandomLocation (AI|Navigation|GetRandomReachablePointinRadius (Transformation|GetActorLocation) 1e+03 0 0)) 0 5.0 false)))

(fn ConstructionScript)